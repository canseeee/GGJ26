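; Behavior Tree task that adds or removes a gameplay tag on the controlled pawn, selected by OperationType.
; On execute, it casts the pawn to ShadowCharacterBase and caches its AbilitySystemComponent, finishing as failed if none is found.
; A second sequence step runs regardless, adding a non-replicated loose tag via the pawn or removing all loose instances from the cached ASC, then finishing successfully.
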(event `self.ReceiveExecuteAI`
  (params (OwnerController :type "AIController Object Reference") (ControlledPawn :type "Pawn Object Reference"))
  (`|ExecutionSequence`
    (:`then_0`
      ;[1 1 1] 检查引用是否有效
      (bind _output_get (set `self.ControlledPawn` ControlledPawn))
      (bind _asshadow_character_base (cast `ShadowCharacterBase` _output_get))
      (bind _returnvalue (`Actor.GetComponentByClass` _asshadow_character_base "/Script/GameplayAbilities.AbilitySystemComponent"))
      (`/Engine/EditorBlueprintResources/StandardMacros.IsValid` _returnvalue
        (:`Is Valid`
          (set `self.ASC` _returnvalue))
        (:`Is Not Valid`
          (`self.FinishExecute` false))))
    (:`then_1`
      (if (== (`self.OperationType`) 0)
        (`AbilitySystemBlueprintLibrary.AddLooseGameplayTags` (`self.ControlledPawn`) (`BlueprintGameplayTagLibrary.MakeGameplayTagContainerFromTag` (`self.GameplayTag`)))
        (`self.FinishExecute` true)
        (else
          (`ShadowAbilitySystemLibrary.RemoveAllLooseGameplayTagFromASC` (`self.ASC`) (`self.GameplayTag`))
          (`self.FinishExecute` true))))))