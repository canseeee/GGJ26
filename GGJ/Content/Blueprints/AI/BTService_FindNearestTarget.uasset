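; Behavior Tree service that finds the tagged actor nearest to the AI-controlled pawn.
; Each AI tick it resets the closest distance to a very large sentinel, gathers all actors with TargetTag and compares their distances to the pawn.
; Each closer actor found is written to the TargetActor Blackboard key, leaving the nearest one stored.
; The key is never cleared, so it keeps its previous value when no actor qualifies.
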(event `self.ReceiveTickAI`
  (params (OwnerController :type "AIController Object Reference") (ControlledPawn :type "Pawn Object Reference") (DeltaSeconds :type "Float (single-precision)"))
  (set `self.ClosestDistance` 99999997952.0)
  (set `self.ControlledActor` ControlledPawn)
  (bind _outactors (`GameplayStatics.GetAllActorsWithTag` (`self.TargetTag`)))
  (for _array_element _outactors
    (bind _returnvalue (`Actor.GetDistanceTo` (`self.ControlledActor`) _array_element))
    (if (< _returnvalue (`self.ClosestDistance`))
      (set `self.ClosestDistance` _returnvalue)
      (`BTFunctionLibrary.SetBlackboardValueAsObject` (`self.TargetActor`) _array_element))))