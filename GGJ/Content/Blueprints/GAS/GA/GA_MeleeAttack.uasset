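; GA_MeleeAttack is a melee attack gameplay ability that damages actors overlapping the avatar's weapon capsule.
; On activation it gets the capsule through CombatInterface, starts waits for Attack.Damage.Start and End, and immediately sets Pawn collision to Ignore.
; The Start event binds the overlap handler, which calls CauseDamage, and switches Pawn collision to Overlap.
; The End event's received output is unwired, and the ability never calls EndAbility.
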(event `self.K2_ActivateAbility`
  (bind _ascombat_interface (cast `CombatInterface` (`self.GetAvatarActorFromActorInfo`)))
  (bind _returnvalue (`CombatInterface.GetWeaponCapsule` _ascombat_interface))
  (bind _output_get (set `self.Capsule` _returnvalue))
  (`AbilityTask_WaitGameplayEvent.WaitGameplayEvent` (struct :`TagName` "Attack.Damage.Start") null
    (:`then`
      (`AbilityTask_WaitGameplayEvent.WaitGameplayEvent` (struct :`TagName` "Attack.Damage.End") null
        (:`then`
          (`PrimitiveComponent.SetCollisionResponseToChannel` (`self.Capsule`) "ECC_Pawn" "ECR_Ignore"))))
    (:`EventReceived`
      (add `PrimitiveComponent.OnComponentBeginOverlap` _output_get (delegate `OnComponentBeginOverlap_事件`))
      (`PrimitiveComponent.SetCollisionResponseToChannel` (`self.Capsule`) "ECC_Pawn" "ECR_Overlap"))))

(event `OnComponentBeginOverlap_事件`
  (params (OverlappedComponent :type "PrimitiveComponent Object Reference") (OtherActor :type "Actor Object Reference") (OtherComp :type "PrimitiveComponent Object Reference") (OtherBodyIndex :type Integer) (bFromSweep :type Boolean) (SweepResult :type "HitResult Structure (by ref)"))
  (`self.CauseDamage` OtherActor))